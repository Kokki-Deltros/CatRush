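; Enemy Blueprint that takes the appearance of a low-poly cat in one of several breed and color skins.
; The construction script maps the Skin variable to a skeletal mesh, resets the pose and applies the shared low-poly cat material.
; The SetSkinPlayer event duplicates that logic so the skin can be reapplied outside construction.
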(event `SetSkinPlayer`
  ;[1 1 1] Set Skin
  ;;[1 1 1] Set SK
  (`SkinnedMeshComponent.SetSkinnedAssetAndUpdate` (`self.Mesh`) (select `/Game/Blueprints/Enemy/Enum_SkinEnemies` (`self.Skin`) :`NewEnumerator2` "/Game/SkeletalMesh/LowPolyCat/Mesh_Cat_Abyss.Mesh_Cat_Abyss" :`NewEnumerator0` "/Game/SkeletalMesh/LowPolyCat/Mesh_Cat_black.Mesh_Cat_black" :`NewEnumerator1` "/Game/SkeletalMesh/LowPolyCat/Mesh_Cat_Black_White.Mesh_Cat_Black_White" :`NewEnumerator3` "/Game/SkeletalMesh/LowPolyCat/Mesh_Cat_Blue.Mesh_Cat_Blue" :`NewEnumerator4` "/Game/SkeletalMesh/LowPolyCat/Mesh_Cat_Bobtail.Mesh_Cat_Bobtail" :`NewEnumerator5` "/Game/SkeletalMesh/LowPolyCat/Mesh_Cat_Brit.Mesh_Cat_Brit" :`NewEnumerator6` "/Game/SkeletalMesh/LowPolyCat/Mesh_Cat_brown.Mesh_Cat_brown" :`NewEnumerator7` "/Game/SkeletalMesh/LowPolyCat/Mesh_Cat_cream.Mesh_Cat_cream" :`NewEnumerator8` "/Game/SkeletalMesh/LowPolyCat/Mesh_Cat_maine.Mesh_Cat_maine" :`NewEnumerator9` "/Game/SkeletalMesh/LowPolyCat/Mesh_Cat_Pers.Mesh_Cat_Pers" :`NewEnumerator10` "/Game/SkeletalMesh/LowPolyCat/Mesh_Cat_Red.Mesh_Cat_Red" :`NewEnumerator11` "/Game/SkeletalMesh/LowPolyCat/Mesh_Cat_Red_White.Mesh_Cat_Red_White" :`NewEnumerator12` "/Game/SkeletalMesh/LowPolyCat/Mesh_Cat_Siamese.Mesh_Cat_Siamese" :`NewEnumerator13` "/Game/SkeletalMesh/LowPolyCat/Mesh_Cat_Sphynx.Mesh_Cat_Sphynx" :`NewEnumerator14` "/Game/SkeletalMesh/LowPolyCat/Mesh_Cat_white.Mesh_Cat_white" :!type "SkeletalMesh Object Reference") true)
  ;;[1 1 1] Set materials
  (`PrimitiveComponent.SetMaterial` (`self.Mesh`) 0 "/Game/Materials/LowPolyCat/Materials/M_LowPoly_Cat.M_LowPoly_Cat"))

(fn `UserConstructionScript`
  ;[1 1 1] Set Skin in Construction
  ;;[1 1 1] Set SK
  (`SkinnedMeshComponent.SetSkinnedAssetAndUpdate` (`self.Mesh`) (select `/Game/Blueprints/Enemy/Enum_SkinEnemies` (`self.Skin`) :`NewEnumerator2` "/Game/SkeletalMesh/LowPolyCat/Mesh_Cat_Abyss.Mesh_Cat_Abyss" :`NewEnumerator0` "/Game/SkeletalMesh/LowPolyCat/Mesh_Cat_black.Mesh_Cat_black" :`NewEnumerator1` "/Game/SkeletalMesh/LowPolyCat/Mesh_Cat_Black_White.Mesh_Cat_Black_White" :`NewEnumerator3` "/Game/SkeletalMesh/LowPolyCat/Mesh_Cat_Blue.Mesh_Cat_Blue" :`NewEnumerator4` "/Game/SkeletalMesh/LowPolyCat/Mesh_Cat_Bobtail.Mesh_Cat_Bobtail" :`NewEnumerator5` "/Game/SkeletalMesh/LowPolyCat/Mesh_Cat_Brit.Mesh_Cat_Brit" :`NewEnumerator6` "/Game/SkeletalMesh/LowPolyCat/Mesh_Cat_brown.Mesh_Cat_brown" :`NewEnumerator7` "/Game/SkeletalMesh/LowPolyCat/Mesh_Cat_cream.Mesh_Cat_cream" :`NewEnumerator8` "/Game/SkeletalMesh/LowPolyCat/Mesh_Cat_maine.Mesh_Cat_maine" :`NewEnumerator9` "/Game/SkeletalMesh/LowPolyCat/Mesh_Cat_Pers.Mesh_Cat_Pers" :`NewEnumerator10` "/Game/SkeletalMesh/LowPolyCat/Mesh_Cat_Red.Mesh_Cat_Red" :`NewEnumerator11` "/Game/SkeletalMesh/LowPolyCat/Mesh_Cat_Red_White.Mesh_Cat_Red_White" :`NewEnumerator12` "/Game/SkeletalMesh/LowPolyCat/Mesh_Cat_Siamese.Mesh_Cat_Siamese" :`NewEnumerator13` "/Game/SkeletalMesh/LowPolyCat/Mesh_Cat_Sphynx.Mesh_Cat_Sphynx" :`NewEnumerator14` "/Game/SkeletalMesh/LowPolyCat/Mesh_Cat_white.Mesh_Cat_white" :!type "SkeletalMesh Object Reference") true)
  ;;[1 1 1] Set materials
  (`PrimitiveComponent.SetMaterial` (`self.Mesh`) 0 "/Game/Materials/LowPolyCat/Materials/M_LowPoly_Cat.M_LowPoly_Cat"))