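; Playground platform segment of a lane-based course that randomly fills itself and chains the next segment.
; On BeginPlay, each of eight three-lane rows gets a random trap with random X offset; movable walls appear only in side lanes.
; The free lanes get a coin or rare multi-coin, plus sometimes a minion spawner.
; Player overlap with SpawnPlatform spawns another segment until the player's platform limit, then the finish.
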(event `self.ReceiveBeginPlay`
  ;[1 1 1] Spawn Traps
  (`self.Spawn Traps` (`self.T_Side2`) (`self.T_Center1`) (`self.T_Side1`))
  (`self.Spawn Traps` (`self.T_Side3`) (`self.T_Center2`) (`self.T_Side4`))
  (`self.Spawn Traps` (`self.T_Side5`) (`self.T_Center3`) (`self.T_Side6`))
  (`self.Spawn Traps` (`self.T_Side7`) (`self.T_Center4`) (`self.T_Side8`))
  (`self.Spawn Traps` (`self.T_Side9`) (`self.T_Center5`) (`self.T_Side10`))
  (`self.Spawn Traps` (`self.T_Side11`) (`self.T_Center6`) (`self.T_Side12`))
  (`self.Spawn Traps` (`self.T_Side13`) (`self.T_Center7`) (`self.T_Side14`))
  (`self.Spawn Traps` (`self.T_Side15`) (`self.T_Center8`) (`self.T_Side16`)))

(event `self.SpawnPlatform.OnComponentBeginOverlap`
  (params (OverlappedComponent :type "PrimitiveComponent Object Reference") (OtherActor :type "Actor Object Reference") (OtherComp :type "PrimitiveComponent Object Reference") (OtherBodyIndex :type Integer) (bFromSweep :type Boolean) (SweepResult :type "HitResult Structure (by ref)"))
  (bind (_returnvalue_location _returnvalue_rotation) (`KismetMathLibrary.BreakTransform` (`SceneComponent.K2_GetComponentToWorld` (`self.Arrow Spawn Location Platform`))))
  (bind (_returnvalue_location_2 _returnvalue_rotation_2) (`KismetMathLibrary.BreakTransform` (`SceneComponent.K2_GetComponentToWorld` (`self.Arrow Spawn Location Platform`))))
  ;[1 1 1] Spawn New plateform
  (bind _asbp_movement_player (cast `/Game/Blueprints/Player/BP_Movement_Player` OtherActor))
  (bind _current_nb_platform (`/Game/Blueprints/Player/BP_Movement_Player.Current_Nb_Platform` _asbp_movement_player))
  (if (< _current_nb_platform (`/Game/Blueprints/Player/BP_Movement_Player.Max_Nb_Platform` _asbp_movement_player))
    (`/Engine/EditorBlueprintResources/StandardMacros.IncrementInt` _current_nb_platform
      (:`  `
        (`|SpawnActorFromClass` "Playground_Level_C" (`KismetMathLibrary.MakeTransform` _returnvalue_location_2 _returnvalue_rotation_2) "Undefined" "OverrideRootScale" null null)))
    (else
      ;;[1 1 1] Spawn Finish
      (`|SpawnActorFromClass` "/Game/Blueprints/Playground/Playground_Finish.Playground_Finish_C" (`KismetMathLibrary.MakeTransform` _returnvalue_location _returnvalue_rotation) "Undefined" "OverrideRootScale" null null))))

(fn `Spawn Coin/AI`
  (params (`Trap 1` :type "ArrowComponent Object Reference (by ref)") (`Trap 2` :type "ArrowComponent Object Reference (by ref)"))
  (locals (RandomTrapPlace :type Integer :default 0))
  (bind _tab_traps (`self.Tab_Traps`))
  (bind (_returnvalue_x _returnvalue_y _returnvalue_z) (`KismetMathLibrary.BreakVector` (`SceneComponent.K2_GetComponentLocation` (`|GetArrayItem` _tab_traps 1))))
  (bind (_returnvalue_x_2 _returnvalue_y_2 _returnvalue_z_2) (`KismetMathLibrary.BreakVector` (`SceneComponent.K2_GetComponentLocation` (`|GetArrayItem` _tab_traps))))
  (`KismetArrayLibrary.Array_Add` _tab_traps `Trap 1`)
  (`KismetArrayLibrary.Array_Add` _tab_traps `Trap 2`)
  (bind _output_get (set `local.RandomTrapPlace` (`KismetMathLibrary.RandomIntegerInRange` 0 1)))
  (if (== (`KismetMathLibrary.RandomIntegerInRange` 1 10) 5)
    (bind _output (`|GetArrayItem` _tab_traps _output_get))
    (bind (_returnvalue_x_3 _returnvalue_y_3 _returnvalue_z_3) (`KismetMathLibrary.BreakVector` (`SceneComponent.K2_GetComponentLocation` _output)))
    (`|SpawnActorFromClass` "/Game/Blueprints/PickUp/BP_MultiCoin.BP_MultiCoin_C" (`KismetMathLibrary.MakeTransform` (`KismetMathLibrary.MakeVector` _returnvalue_x_3 _returnvalue_y_3 _returnvalue_z_3)) "Undefined" "OverrideRootScale" null null)
    (else
      (bind (_returnvalue_x_4 _returnvalue_y_4 _returnvalue_z_4) (`KismetMathLibrary.BreakVector` (`SceneComponent.K2_GetComponentLocation` _output)))
      (`|SpawnActorFromClass` "/Game/Blueprints/PickUp/BP_Coin.BP_Coin_C" (`KismetMathLibrary.MakeTransform` (`KismetMathLibrary.MakeVector` _returnvalue_x_4 _returnvalue_y_4 _returnvalue_z_4)) "Undefined" "OverrideRootScale" null null)))
  (if (== _output_get 0)
    (if (== (`KismetMathLibrary.RandomIntegerInRange` 1 3) 2)
      (if (== (`KismetMathLibrary.RandomIntegerInRange` 1 3) 2)
        (`|SpawnActorFromClass` "/Game/Blueprints/Player/BP_Spawn_Player_Minion.BP_Spawn_Player_Minion_C" (`KismetMathLibrary.MakeTransform` (`KismetMathLibrary.MakeVector` _returnvalue_x _returnvalue_y _returnvalue_z)) "Undefined" "OverrideRootScale" null 150.0 (`KismetMathLibrary.RandomIntegerInRange` 2 4) null)
        (else
          (`|SpawnActorFromClass` "/Game/Blueprints/Player/BP_Spawn_Player_Minion.BP_Spawn_Player_Minion_C" (`KismetMathLibrary.MakeTransform` (`KismetMathLibrary.MakeVector` _returnvalue_x _returnvalue_y _returnvalue_z)) "Undefined" "OverrideRootScale" null 150.0 1 null))))
    (elif (== (`KismetMathLibrary.RandomIntegerInRange` 1 3) 2)
      (if (== (`KismetMathLibrary.RandomIntegerInRange` 1 3) 2)
        (`|SpawnActorFromClass` "/Game/Blueprints/Player/BP_Spawn_Player_Minion.BP_Spawn_Player_Minion_C" (`KismetMathLibrary.MakeTransform` (`KismetMathLibrary.MakeVector` _returnvalue_x_2 _returnvalue_y_2 _returnvalue_z_2)) "Undefined" "OverrideRootScale" null 150.0 (`KismetMathLibrary.RandomIntegerInRange` 2 4) null)
        (else
          (`|SpawnActorFromClass` "/Game/Blueprints/Player/BP_Spawn_Player_Minion.BP_Spawn_Player_Minion_C" (`KismetMathLibrary.MakeTransform` (`KismetMathLibrary.MakeVector` _returnvalue_x_2 _returnvalue_y_2 _returnvalue_z_2)) "Undefined" "OverrideRootScale" null 150.0 1 null)))))
  (`KismetArrayLibrary.Array_Clear` _tab_traps))

(fn `Spawn Traps`
  (params (`Right Trap` :type "ArrowComponent Object Reference") (`Center Trap` :type "ArrowComponent Object Reference") (`Left Trap` :type "ArrowComponent Object Reference"))
  (locals (`Rand Index Trap Place` :type Integer :default 0) (`Rand Index Trap Class` :type Integer :default 0))
  (bind _output_get (set `local.Rand Index Trap Place` (`KismetMathLibrary.RandomIntegerInRange` 0 2)))
  (switch `int` _output_get
    (:`0`
      (`self.Spawn Coin/AI` `Center Trap` `Left Trap`)
      ;[1 1 1] Trap on the right
      (bind _output_get_2 (set `local.Rand Index Trap Class` (`KismetMathLibrary.RandomIntegerInRange` 0 2)))
      (switch `int` _output_get_2
        (:`0`
          (bind _returnvalue (select `int` _output_get :`0` `Right Trap` :`1` `Center Trap` :`2` `Left Trap`))
          (bind (_returnvalue_x _returnvalue_y _returnvalue_z) (`KismetMathLibrary.BreakVector` (`SceneComponent.K2_GetComponentLocation` _returnvalue)))
          (`|SpawnActorFromClass` "/Game/Blueprints/Traps/BP_Traps_Wall.BP_Traps_Wall_C" (`KismetMathLibrary.MakeTransform` (`KismetMathLibrary.MakeVector` (+ (`KismetMathLibrary.RandomFloatInRange` 0.0 (`self.Max Range Loc Traps`)) _returnvalue_x) _returnvalue_y _returnvalue_z)) "Undefined" "OverrideRootScale" null null))
        (:`1`
          (bind (_returnvalue_x_2 _returnvalue_y_2 _returnvalue_z_2) (`KismetMathLibrary.BreakVector` (`SceneComponent.K2_GetComponentLocation` _returnvalue)))
          (`|SpawnActorFromClass` "/Game/Blueprints/Traps/BP_Traps_Spikes.BP_Traps_Spikes_C" (`KismetMathLibrary.MakeTransform` (`KismetMathLibrary.MakeVector` (+ (`KismetMathLibrary.RandomFloatInRange` 0.0 (`self.Max Range Loc Traps`)) _returnvalue_x_2) _returnvalue_y_2 _returnvalue_z_2)) "Undefined" "OverrideRootScale" null 1.0 1.0 5.0 null))
        (:`2`
          (bind (_returnvalue_x_3 _returnvalue_y_3 _returnvalue_z_3) (`KismetMathLibrary.BreakVector` (`SceneComponent.K2_GetComponentLocation` _returnvalue)))
          (`|SpawnActorFromClass` "/Game/Blueprints/Traps/BP_Traps_Movable_Wall.BP_Traps_Movable_Wall_C" (`KismetMathLibrary.MakeTransform` (`KismetMathLibrary.MakeVector` (+ (`KismetMathLibrary.RandomFloatInRange` 0.0 (`self.Max Range Loc Traps`)) _returnvalue_x_3) _returnvalue_y_3 _returnvalue_z_3) (struct :`Yaw` -90.0)) "Undefined" "OverrideRootScale" null 1.0 1.0 180.0 null))))
    (:`1`
      (`self.Spawn Coin/AI` `Right Trap` `Left Trap`)
      ;[1 1 1] Trap at the center
      (bind _output_get_3 (set `local.Rand Index Trap Class` (`KismetMathLibrary.RandomIntegerInRange` 0 1)))
      (switch `int` _output_get_3
        (:`0`
          (bind (_returnvalue_x_4 _returnvalue_y_4 _returnvalue_z_4) (`KismetMathLibrary.BreakVector` (`SceneComponent.K2_GetComponentLocation` _returnvalue)))
          (`|SpawnActorFromClass` "/Game/Blueprints/Traps/BP_Traps_Wall.BP_Traps_Wall_C" (`KismetMathLibrary.MakeTransform` (`KismetMathLibrary.MakeVector` (+ (`KismetMathLibrary.RandomFloatInRange` 0.0 (`self.Max Range Loc Traps`)) _returnvalue_x_4) _returnvalue_y_4 _returnvalue_z_4)) "Undefined" "OverrideRootScale" null null))
        (:`1`
          (bind (_returnvalue_x_5 _returnvalue_y_5 _returnvalue_z_5) (`KismetMathLibrary.BreakVector` (`SceneComponent.K2_GetComponentLocation` _returnvalue)))
          (`|SpawnActorFromClass` "/Game/Blueprints/Traps/BP_Traps_Spikes.BP_Traps_Spikes_C" (`KismetMathLibrary.MakeTransform` (`KismetMathLibrary.MakeVector` (+ (`KismetMathLibrary.RandomFloatInRange` 0.0 (`self.Max Range Loc Traps`)) _returnvalue_x_5) _returnvalue_y_5 _returnvalue_z_5)) "Undefined" "OverrideRootScale" null 1.0 1.0 5.0 null))
        (:`2`
          (bind (_returnvalue_x_6 _returnvalue_y_6 _returnvalue_z_6) (`KismetMathLibrary.BreakVector` (`SceneComponent.K2_GetComponentLocation` _returnvalue)))
          (`|SpawnActorFromClass` "/Game/Blueprints/Traps/BP_Traps_Movable_Wall.BP_Traps_Movable_Wall_C" (`KismetMathLibrary.MakeTransform` (`KismetMathLibrary.MakeVector` (+ (`KismetMathLibrary.RandomFloatInRange` 0.0 (`self.Max Range Loc Traps`)) _returnvalue_x_6) _returnvalue_y_6 _returnvalue_z_6)) "Undefined" "OverrideRootScale" null 1.0 1.0 180.0 null))))
    (:`2`
      (`self.Spawn Coin/AI` `Right Trap` `Center Trap`)
      ;[1 1 1] Trap on the left
      (bind _output_get_4 (set `local.Rand Index Trap Class` (`KismetMathLibrary.RandomIntegerInRange` 0 2)))
      (switch `int` _output_get_4
        (:`0`
          (bind (_returnvalue_x_7 _returnvalue_y_7 _returnvalue_z_7) (`KismetMathLibrary.BreakVector` (`SceneComponent.K2_GetComponentLocation` _returnvalue)))
          (`|SpawnActorFromClass` "/Game/Blueprints/Traps/BP_Traps_Wall.BP_Traps_Wall_C" (`KismetMathLibrary.MakeTransform` (`KismetMathLibrary.MakeVector` (+ (`KismetMathLibrary.RandomFloatInRange` 0.0 (`self.Max Range Loc Traps`)) _returnvalue_x_7) _returnvalue_y_7 _returnvalue_z_7)) "Undefined" "OverrideRootScale" null null))
        (:`1`
          (bind (_returnvalue_x_8 _returnvalue_y_8 _returnvalue_z_8) (`KismetMathLibrary.BreakVector` (`SceneComponent.K2_GetComponentLocation` _returnvalue)))
          (`|SpawnActorFromClass` "/Game/Blueprints/Traps/BP_Traps_Spikes.BP_Traps_Spikes_C" (`KismetMathLibrary.MakeTransform` (`KismetMathLibrary.MakeVector` (+ (`KismetMathLibrary.RandomFloatInRange` 0.0 (`self.Max Range Loc Traps`)) _returnvalue_x_8) _returnvalue_y_8 _returnvalue_z_8)) "Undefined" "OverrideRootScale" null 1.0 1.0 5.0 null))
        (:`2`
          (bind (_returnvalue_x_9 _returnvalue_y_9 _returnvalue_z_9) (`KismetMathLibrary.BreakVector` (`SceneComponent.K2_GetComponentLocation` _returnvalue)))
          (`|SpawnActorFromClass` "/Game/Blueprints/Traps/BP_Traps_Movable_Wall.BP_Traps_Movable_Wall_C" (`KismetMathLibrary.MakeTransform` (`KismetMathLibrary.MakeVector` (+ (`KismetMathLibrary.RandomFloatInRange` 0.0 (`self.Max Range Loc Traps`)) _returnvalue_x_9) _returnvalue_y_9 _returnvalue_z_9) (struct :`Yaw` 90.0)) "Undefined" "OverrideRootScale" null 1.0 1.0 180.0 null))))))

(fn `UserConstructionScript`)