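; Finish trigger actor for the Playground level that ends the run when a BP_Movement_Player overlaps it.
; On overlap it loops the jump animation on the player mesh, stops movement immediately and zeroes the walk speed.
; It then swaps the player's HUD widget for a newly created WG_Finish_Menu and prints the walk speed as debug output.
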(event `self.ReceiveActorBeginOverlap`
  (params (OtherActor :type "Actor Object Reference"))
  (bind _asbp_movement_player (cast `/Game/Blueprints/Player/BP_Movement_Player` OtherActor))
  (`SkeletalMeshComponent.PlayAnimation` (`Character.Mesh` _asbp_movement_player) "/Game/Animations/Player/Anim_Jump.Anim_Jump" true)
  (bind _charactermovement (`Character.CharacterMovement` _asbp_movement_player))
  (`MovementComponent.StopMovementImmediately` _charactermovement)
  (set `CharacterMovementComponent.MaxWalkSpeed` 0.0 _charactermovement)
  (`Widget.RemoveFromParent` (`/Game/Blueprints/Player/BP_Movement_Player.WG_Player_Ref` _asbp_movement_player))
  (bind _returnvalue (`|CreateWidget` "/Game/Blueprints/Widget/WG_Finish_Menu.WG_Finish_Menu_C"))
  (bind _output_get (set `self.WG_Finish_Ref` _returnvalue))
  (`UserWidget.AddToViewport` _output_get 0)
  (`KismetSystemLibrary.PrintString` (`KismetStringLibrary.Conv_DoubleToString` (`CharacterMovementComponent.MaxWalkSpeed` _charactermovement)) true true (struct :`G` 0.66 :`B` 1.0 :`A` 1.0) 100.0))

(fn `UserConstructionScript`)