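; BP_IA_Player is a minion that wears the player's skin and, once it joins, moves along with BP_Movement_Player.
; An inactive minion touched by an active one activates its Spawner, while JoinPlayer activates the minion and registers it with the player.
; Active minions copy the player's velocity and rotation each tick, and Replace teleports them onto the player.
; Unless the player is invincible, Death unregisters and destroys it with blood effects.
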(event `self.ReceiveBeginPlay`
  ;[1 1 1] Begin Play
  (bind _returnvalue (`GameplayStatics.GetActorOfClass` "/Game/Blueprints/Player/BP_Movement_Player.BP_Movement_Player_C"))
  (bind _output_get (set `self.Ref Player` _returnvalue))
  (`KismetSystemLibrary.Delay` 0.5)
  (`/Game/Blueprints/Player/BP_Movement_Player.SetSkinPlayer` _output_get (`/Game/Blueprints/Player/BP_Movement_Player.Skin` _output_get) (`self.Mesh`)))

(event `Replace`
  (bind _ref_player (`self.Ref Player`))
  (`self.K2_TeleportTo` self (`self.K2_GetActorLocation` _ref_player) (`self.K2_GetActorRotation` _ref_player)))

(event `self.ReceiveTick`
  (params (DeltaSeconds :type "Float (single-precision)"))
  (bind _ref_player (`self.Ref Player`))
  ;[1 1 1] Tick - Deplacement
  (if (`self.IsActive`)
    (`PrimitiveComponent.SetPhysicsLinearVelocity` (`self.CapsuleComponent`) (`self.GetVelocity` _ref_player) false "None")
    (`self.K2_SetActorRotation` (`self.K2_GetActorRotation` _ref_player))))

(event `self.CapsuleComponent.OnComponentBeginOverlap`
  (params (OverlappedComponent :type "PrimitiveComponent Object Reference") (OtherActor :type "Actor Object Reference") (OtherComp :type "PrimitiveComponent Object Reference") (OtherBodyIndex :type Integer) (bFromSweep :type Boolean) (SweepResult :type "HitResult Structure (by ref)"))
  (bind _spawner (`self.Spawner`))
  ;[1 1 1] Join Player?
  ;;[1 1 1] Detect
  (if (not (`self.IsActive`))
    (bind _asbp_ia_player (cast `/Game/Blueprints/Player/BP_IA_Player` OtherActor))
    (if (`/Game/Blueprints/Player/BP_IA_Player.IsActive` _asbp_ia_player)
      (`/Engine/EditorBlueprintResources/StandardMacros.IsValid` _spawner
        (:`Is Valid`
          (`/Game/Blueprints/Player/BP_Spawn_Player_Minion.Activate` _spawner))))))

(event `JoinPlayer`
  ;[1 1 1] Join Player?
  ;;[1 1 1] JoinPlayer
  (`/Engine/EditorBlueprintResources/StandardMacros.DoOnce` false
    (:`Completed`
      (set `self.IsActive` true)
      (`/Game/Blueprints/Player/BP_Movement_Player.AddMinion` (`self.Ref Player`) self))))

(event `Death`
  (bind _returnvalue_location (`KismetMathLibrary.BreakTransform` (`self.GetTransform` self)))
  ;[1 1 1] Death
  (if (not (`/Game/Blueprints/Player/BP_Movement_Player.Invincible` (cast `/Game/Blueprints/Player/BP_Movement_Player` (`GameplayStatics.GetPlayerCharacter` 0) :!pure true)))
    (`/Engine/EditorBlueprintResources/StandardMacros.DoOnce` false :!label _label
      (:`Completed`
        (`/Game/Blueprints/Player/BP_Movement_Player.RemoveMinion` (`self.Ref Player`) self)
        (`NiagaraFunctionLibrary.SpawnSystemAtLocation` "/Game/Niagara/System/NS_BloodSplash.NS_BloodSplash" _returnvalue_location)
        (if (`self.IsActive`)
          (`GameplayStatics.PlaySoundAtLocation` "/Game/Sounds/Squirt_Cue.Squirt_Cue" _returnvalue_location (struct) 1.0 1.0 0.0 null null null))
        (`self.K2_DestroyActor`)))
    (else
      (goto _label :!via `Reset`))))

(fn `UserConstructionScript`)