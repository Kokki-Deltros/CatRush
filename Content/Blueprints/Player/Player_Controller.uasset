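; Player controller Blueprint that saves and loads the player's progress (current level, skin and coins) through a single save slot.
; LoadGame loads an existing TheSaveGame asynchronously and copies its struct into BP_Player, or calls NewGame to create an empty save object if none exists.
; SaveGame writes BP_Player's values back into the struct and saves it to the slot, with debug prints marking the steps.
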(event `Load Game`
  (bind _asbp_player (cast `/Game/Blueprints/Player/BP_Player` (`GameplayStatics.GetPlayerCharacter` 0) :!pure true))
  (`KismetSystemLibrary.PrintString` "AVANT TOUT")
  (bind _returnvalue (`GameplayStatics.DoesSaveGameExist` "SaveGame"))
  (if _returnvalue
    (`KismetSystemLibrary.PrintString` "AVANT SAVE")
    (bind _savegame (`AsyncActionHandleSaveGame.AsyncLoadGameFromSlot` "SaveGame")
      (:`then`
        (bind _asthe_save_game (cast `/Game/Blueprints/Save/TheSaveGame` _savegame))
        (bind _output_get (set `self.TheSaveGame_Ref` _asthe_save_game))
        (bind (_struct_save_level _struct_save_skin _struct_save_coin) (break `/Game/Blueprints/Save/Struct_Save` (`/Game/Blueprints/Save/TheSaveGame.Struct_Save` _output_get)))
        (set `/Game/Blueprints/Player/BP_Player.Current_Level` _struct_save_level _asbp_player)
        (set `/Game/Blueprints/Player/BP_Player.Skin` _struct_save_skin _asbp_player)
        (set `/Game/Blueprints/Player/BP_Player.Coin` _struct_save_coin _asbp_player)
        (`KismetSystemLibrary.PrintString` "LOAD SAVE")))
    (else
      (`self.New Game`))))

(event `New Game`
  (bind _returnvalue (`GameplayStatics.CreateSaveGameObject` "/Game/Blueprints/Save/TheSaveGame.TheSaveGame_C"))
  (set `self.TheSaveGame_Ref` _returnvalue)
  (`KismetSystemLibrary.PrintString` "NEW SAVE"))

(event `Save Game`
  (bind _asbp_player (cast `/Game/Blueprints/Player/BP_Player` (`GameplayStatics.GetPlayerCharacter` 0) :!pure true))
  (set `/Game/Blueprints/Save/TheSaveGame.Struct_Save` (make `/Game/Blueprints/Save/Struct_Save` (`/Game/Blueprints/Player/BP_Player.Current_Level` _asbp_player) (`/Game/Blueprints/Player/BP_Player.Skin` _asbp_player) (`/Game/Blueprints/Player/BP_Player.Coin` _asbp_player)) (`self.TheSaveGame_Ref`))
  (`GameplayStatics.SaveGameToSlot` (`self.TheSaveGame_Ref`) "SaveGame")
  (`KismetSystemLibrary.PrintString` "SAVE"))

(fn `UserConstructionScript`)