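; BP_Spawn_Player_Minion is a world spawner that creates friendly AI minions who later join the player.
; On BeginPlay it spawns the set number of BP_IA_Player minions near the sphere's center with small random offsets, passing the player's skin and itself as spawner.
; Activate tells each stored minion to join the player, then destroys the spawner.
; The construction script sizes the sphere from the Radius variable.
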(event `self.ReceiveBeginPlay`
  (bind (_returnvalue_location _returnvalue_rotation _returnvalue_scale) (`KismetMathLibrary.BreakTransform` (`SceneComponent.K2_GetComponentToWorld` (`self.Sphere`))))
  ;[1 1 1] SpawnIA
  (bind _returnvalue (`GameplayStatics.GetActorOfClass` "/Game/Blueprints/Player/BP_Movement_Player.BP_Movement_Player_C"))
  (bind _output_get (set `self.RefPlayer` _returnvalue))
  (if (> (`self.NumberOfMinions`) 0)
    (for _ (range (`self.NumberOfMinions`))
      (bind _returnvalue_2 (`|SpawnActorFromClass` "/Game/Blueprints/Player/BP_IA_Player.BP_IA_Player_C" (`KismetMathLibrary.MakeTransform` (+ _returnvalue_location (`KismetMathLibrary.MakeVector` (`KismetMathLibrary.RandomFloatInRange` -50.0 50.0) (`KismetMathLibrary.RandomFloatInRange` -50.0 50.0) 20.0)) _returnvalue_rotation _returnvalue_scale) "Undefined" "OverrideRootScale" null (`/Game/Blueprints/Player/BP_Movement_Player.Skin` _output_get) false self null))
      (`KismetArrayLibrary.Array_Add` (`self.RefMinion`) _returnvalue_2))))

(event `Activate`
  ;[1 1 1] IA Join player
  (for _array_element (`self.RefMinion`)
    (`/Game/Blueprints/Player/BP_IA_Player.JoinPlayer` _array_element))
  (`self.K2_DestroyActor`))

(fn `UserConstructionScript`
  (`SphereComponent.SetSphereRadius` (`self.Sphere`) (`self.Radius`) false))